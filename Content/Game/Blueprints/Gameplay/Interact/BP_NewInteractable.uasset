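; Interactable actor that a Character can pick up, carry and launch on release.
; BeginPlay links its mesh and interact widget to a Highlight component, and it always reports itself as interactable.
; Starting interaction makes capsule and sphere ignore each other's actors when moving, attaches it to the Character and deactivates the highlight.
; Finishing detaches it and activates ProjectileMovement along the interactor's forward vector, without restoring collision or highlight.
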(event `self.ReceiveBeginPlay`
  (bind _highlight (`self.Highlight`))
  (`HighlightComponent.SetMeshComponent` _highlight (`self.MainMesh`))
  (`HighlightComponent.SetWidgetComponent` _highlight (`self.InteractWidget`)))

(event `self.StartInteraction`
  (params (ActorInteracting :type "Actor Object Reference"))
  (bind _ascharacter (cast `Character` ActorInteracting))
  (`PrimitiveComponent.IgnoreActorWhenMoving` (`Character.CapsuleComponent` _ascharacter) self true)
  (`PrimitiveComponent.IgnoreActorWhenMoving` (`self.Sphere`) ActorInteracting true)
  (`self.K2_AttachToActor` ActorInteracting "None" "SnapToTarget" "SnapToTarget" "KeepRelative")
  (`HighlightComponent.DeactivateHighlight` (`self.Highlight`)))

(event `self.FinishInteraction`
  (params (ActorInteracting :type "Actor Object Reference"))
  (bind _projectilemovement (`self.ProjectileMovement`))
  (`self.K2_DetachFromActor` "KeepWorld" "KeepWorld" "KeepWorld")
  (`ActorComponent.Activate` _projectilemovement false)
  (set `MovementComponent.Velocity` (* (`self.GetActorForwardVector` ActorInteracting) 1000.0) _projectilemovement))

(fn `CanBeInteracted`
  (params (ActorInteracting :type "Actor Object Reference"))
  (returns (ReturnValue :type Boolean))
  (return true))

(fn `UserConstructionScript`)