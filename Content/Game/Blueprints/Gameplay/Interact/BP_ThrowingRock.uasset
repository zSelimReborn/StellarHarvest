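; Throwable rock interactable that a character picks up and throws to stun whatever it hits.
; Starting interaction attaches it to the character's "Rock"-tagged component, or to the actor as fallback, with mutual move-ignore to avoid collisions.
; Finishing interaction detaches it and launches it along the thrower's forward vector via ProjectileMovement.
; Blocking bounces stun actors with a StunHandlerComponent and spawn an explosion; stopping restores collision and interactability.
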(event `self.ReceiveBeginPlay`
  (bind _highlight (`self.Highlight`))
  (`HighlightComponent.SetMeshComponent` _highlight (`self.MainMesh`))
  (`HighlightComponent.SetWidgetComponent` _highlight (`self.InteractWidget`))
  (`MovementComponent.SetUpdatedComponent` (`self.RotatingMovement`) (`self.MainMesh`)))

(event `self.StartInteraction`
  (params (ActorInteracting :type "Actor Object Reference"))
  (bind _returnvalue (`self.FindComponentByTag` ActorInteracting "/Script/Engine.SceneComponent" "Rock"))
  (bind _ascharacter (cast `Character` ActorInteracting))
  (set `self.Actor Interacting` _ascharacter)
  (`PrimitiveComponent.IgnoreActorWhenMoving` (`Character.CapsuleComponent` _ascharacter) self true)
  (`PrimitiveComponent.IgnoreActorWhenMoving` (`self.Sphere`) ActorInteracting true)
  (`/Engine/EditorBlueprintResources/StandardMacros.IsValid` _returnvalue
    (:`Is Valid`
      (`self.K2_AttachToComponent` _returnvalue "None" "SnapToTarget" "SnapToTarget" "KeepRelative"))
    (:`Is Not Valid`
      (`self.K2_AttachToActor` ActorInteracting "None" "SnapToTarget" "SnapToTarget" "KeepRelative")))
  (`HighlightComponent.DeactivateHighlight` (`self.Highlight`))
  (set `self.bCanBeInteracted` false))

(event `self.FinishInteraction`
  (params (ActorInteracting :type "Actor Object Reference"))
  (bind _projectilemovement (`self.ProjectileMovement`))
  (`self.K2_DetachFromActor` "KeepWorld" "KeepWorld" "KeepWorld")
  (`MovementComponent.SetUpdatedComponent` _projectilemovement (`self.Sphere`))
  (`ActorComponent.Activate` _projectilemovement false)
  (set `MovementComponent.Velocity` (* (`self.GetActorForwardVector` ActorInteracting) 2000.0) _projectilemovement))

(event `self.ProjectileMovement.OnProjectileStop`
  (params (ImpactResult :type "HitResult Structure (by ref)"))
  (bind _actor_interacting (`self.Actor Interacting`))
  (`/Engine/EditorBlueprintResources/StandardMacros.IsValid` _actor_interacting
    (:`Is Valid`
      (`PrimitiveComponent.ClearMoveIgnoreActors` (`Character.CapsuleComponent` _actor_interacting))
      (`PrimitiveComponent.ClearMoveIgnoreActors` (`self.Sphere`))
      (set `self.Actor Interacting` null)
      (`ActorComponent.Deactivate` (`self.ProjectileMovement`))
      (set `self.bCanBeInteracted` true))))

(event `self.ProjectileMovement.OnProjectileBounce`
  (params (ImpactResult :type "HitResult Structure (by ref)") (ImpactVelocity :type "Vector Structure (by ref)"))
  (if ImpactResult_bBlockingHit
    (`self.TryApplyStun` ImpactResult_HitActor ImpactResult_Location)))

(fn `CanBeInteracted`
  (params (ActorInteracting :type "Actor Object Reference"))
  (returns (ReturnValue :type Boolean))
  (return (`self.bCanBeInteracted`)))

(fn `TryApplyStun`
  (params (Actor :type "Actor Object Reference") (ImpactLocation :type "Vector Structure"))
  (bind _returnvalue (`self.GetComponentByClass` Actor "/Script/StellarHarvest.StunHandlerComponent"))
  (`/Engine/EditorBlueprintResources/StandardMacros.IsValid` Actor
    (:`Is Valid`
      (`/Engine/EditorBlueprintResources/StandardMacros.IsValid` _returnvalue
        (:`Is Valid`
          (`StunHandlerComponent.Apply` _returnvalue 0.0)
          (`GameplayStatics.SpawnEmitterAtLocation` "/Game/StarterContent/Particles/P_Explosion.P_Explosion" ImpactLocation))))))

(fn `UserConstructionScript`)