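; Playable space tractor character Blueprint that supplies the visual, audio and rumble feedback for its abilities and countermeasure.
; The countermeasure component drives either an instantly shown force field sphere or a ground circle grown on Tick from elapsed over total duration, depending on stun mode.
; The primary ability toggles boost particles and controller rumble.
; The secondary ability cloaks body and arms by swapping in an invisible material, restoring materials cached at BeginPlay.
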(event `self.ReceiveBeginPlay`
  (`TransformAnimComponent.SetUpdatedComponent` (`self.Transform Anim Component`) (`self.SpaceTractorArms`))
  (`CounterMeasureComponent.SetTriggerVolume` (`self.CounterMeasure`) (`self.Counter Measure Volume`))
  (`self.StoreTractorMaterials`))

(event `self.ReceiveTick`
  (params (DeltaSeconds :type "Float (single-precision)"))
  (`self.UpdateCounterMeasureScale`))

(event `self.CounterMeasure.OnUseCounterMeasureDelegate`
  (params (CurrentAmount :type Integer))
  (`GameplayStatics.PlaySoundAtLocation` "/Engine/VREditor/Sounds/UI/Dockable_Window_Open.Dockable_Window_Open" (`self.K2_GetActorLocation`) (struct) 1.0 1.0 0.0 null null null null)
  (switch `EStunDealMode` (`CounterMeasureComponent.GetStunMode` (`self.CounterMeasure`))
    (:`ESDM_Instant`
      (`SceneComponent.SetVisibility` (`self.Force Field Sphere`) true true))
    (:`ESDM_Gradual`
      (`SceneComponent.SetRelativeScale3D` (`self.Counter Measure Circle`) (0.0 0.0 1.0))
      (set `self.bScalingCounterMeasure` true))))

(event `self.CounterMeasure.OnFinishDelegate`
  (switch `EStunDealMode` (`CounterMeasureComponent.GetStunMode` (`self.CounterMeasure`))
    (:`ESDM_Instant`
      (`SceneComponent.SetVisibility` (`self.Force Field Sphere`) false true))
    (:`ESDM_Gradual`
      (`SceneComponent.SetRelativeScale3D` (`self.Counter Measure Circle`) (0.0 0.0 1.0))
      (set `self.bScalingCounterMeasure` false))))

(event `self.CounterMeasure.OnCooldownFinishedDelegate`)

(event `self.Ability Component.OnPrimaryAbilityApplied`
  (params (Ability :type "EffectAbility Object Reference"))
  ;[1 1 1] Primary Ability
  (`ActorComponent.Activate` (`self.Boost Particle`) false)
  (bind _asplayer_controller (cast `PlayerController` (`self.GetController`)))
  (`PlayerController.PlayDynamicForceFeedback` _asplayer_controller 0.5 -1.0 false true false true :!label _label))

(event `self.Ability Component.OnPrimaryAbilityRemoved`
  (params (Ability :type "EffectAbility Object Reference"))
  ;[1 1 1] Primary Ability
  (`ActorComponent.Deactivate` (`self.Boost Particle`))
  (goto _label :!via `Stop`))

(event `self.Ability Component.OnPrimaryAbilityAvailable`
  (params (Ability :type "EffectAbility Object Reference"))
  ;[1 1 1] Primary Ability
  (`GameplayStatics.PlaySound2D` "/Engine/VREditor/Sounds/UI/Camera_Shutter.Camera_Shutter" 1.0 1.0 0.0 null null))

(event `self.Ability Component.OnSecondaryAbilityApplied`
  (params (Ability :type "EffectAbility Object Reference"))
  ;[1 1 1] Secondary Ability
  (`self.SetTractorInvisible`))

(event `self.Ability Component.OnSecondaryAbilityRemoved`
  (params (Ability :type "EffectAbility Object Reference"))
  ;[1 1 1] Secondary Ability
  (`self.SetTractorVisible`))

(event `self.Ability Component.OnSecondaryAbilityAvailable`
  (params (Ability :type "EffectAbility Object Reference"))
  ;[1 1 1] Secondary Ability
  (`GameplayStatics.PlaySound2D` "/Engine/VREditor/Sounds/UI/Click_on_Button.Click_on_Button" 1.0 1.0 0.0 null null))

(fn `SetTractorInvisible`
  (for (_ _array_index) (`MeshComponent.GetMaterials` (`self.SpaceTractorBody`))
    (`PrimitiveComponent.SetMaterial` (`self.SpaceTractorBody`) _array_index "/Game/Game/Assets/Material/Cloak/M_Cloak_Invisible.M_Cloak_Invisible"))
  (for (_ _array_index_2) (`MeshComponent.GetMaterials` (`self.SpaceTractorArms`))
    (`PrimitiveComponent.SetMaterial` (`self.SpaceTractorArms`) _array_index_2 "/Game/Game/Assets/Material/Cloak/M_Cloak_Invisible.M_Cloak_Invisible")))

(fn `SetTractorVisible`
  (for (_array_element _array_index) (`self.TractorBodyMaterials`)
    (`PrimitiveComponent.SetMaterial` (`self.SpaceTractorBody`) _array_index _array_element))
  (for (_array_element_2 _array_index_2) (`self.TractorArmMaterials`)
    (`PrimitiveComponent.SetMaterial` (`self.SpaceTractorArms`) _array_index_2 _array_element_2)))

(fn `StoreTractorMaterials`
  (set `self.TractorBodyMaterials` (`MeshComponent.GetMaterials` (`self.SpaceTractorBody`)))
  (set `self.TractorArmMaterials` (`MeshComponent.GetMaterials` (`self.SpaceTractorArms`))))

(fn `UpdateCounterMeasureScale`
  (bind _countermeasure (`self.CounterMeasure`))
  (if (`self.bScalingCounterMeasure`)
    (`SceneComponent.SetRelativeScale3D` (`self.Counter Measure Circle`) (`KismetMathLibrary.VLerp` (0.0 0.0 1.0) (10.9875 10.9875 1.0) (/ (`CounterMeasureComponent.GetCurrentDuration` _countermeasure) (`CounterMeasureComponent.GetDuration` _countermeasure))))))

(fn `UserConstructionScript`)