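; BP_StellarHarvestGameMode is the game mode for Stellar Harvest, holding an unfinished end-state test marked as not working.
; Its BeginPlay and Tick events are empty.
; Two disconnected chains remain: one pauses the game and shows WBP_GameMenu with the mouse cursor.
; The other would quit the game once the player pawn's CrystalCollectorComponent count reaches CrystalsNeededtoComplete.
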(event `self.ReceiveBeginPlay`)

(event `self.ReceiveTick`
  (params (DeltaSeconds :type "Float (single-precision)"))
  ;[1 1 1] Gamemode End State TEST - not working
)

(fn `UserConstructionScript`)